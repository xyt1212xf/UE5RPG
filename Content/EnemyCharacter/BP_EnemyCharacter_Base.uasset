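; Base enemy character Blueprint that plays a random entry montage on spawn, if any are set, and runs the death sequence.
; On death it pauses animation, disables capsule collision, removes enemy widgets and async-loads a Niagara dissolve effect tinted from the mesh material.
; A timeline scaled to TotalDissolveTime dissolves body and weapon, then destroys the weapon, triggers the SpawnStone ability and destroys itself after a delay.
; An unused reverse-dissolve entry effect remains disconnected.
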(event EventBeginPlay
  (bind _entrymontagetoplay (Variables|Default|GetEntryMontageToPlay))
  (if (Utilities|Array|IsNotEmpty _entrymontagetoplay)
    (Animation|PlayAnimMontage (.OutItem (Utilities|Array|Random _entrymontagetoplay)) 1.0 "None")))

(event Collision|EventActorBeginOverlap
  (params (OtherActor :type Actor%20Object%20Reference)))

(event EventTick
  (params (DeltaSeconds :type Float%20%28single-precision%29)))

(event EventOnEnemyDied
  (params (DissolveNiagaraSystem :type Niagara%20System%20Soft%20Object%20Reference))
  (bind _enemycombatcomponentptr (Variables|Default|GetEnemyCombatComponentPtr))
  (bind _enemycombatcomponentptr_2 (Variables|Default|GetEnemyCombatComponentPtr))
  (bind _mesh (Variables|Character|GetMesh))
  (bind _returnvalue (Class|PawnCombatComponent|GetCharacterCurrentEquippedWeapon _enemycombatcomponentptr))
  (bind _returnvalue_2 (Class|PawnCombatComponent|GetCharacterCurrentEquippedWeapon _enemycombatcomponentptr_2))
  (Utilities|FlowControl|Sequence
    (:then_0
      (Variables|/Script/Engine.SkeletalMeshComponent|SetbPauseAnims (Variables|Character|GetMesh) true)
      (Collision|SetCollisionEnabled (Variables|Default|GetCapsuleComponent) "NoCollision"))
    (:then_1
      (Class|EnemyUIComponent|RemoveEnemyDrawnWidgetsifAny (Variables|Default|GetEnemyUIComponent)))
    (:then_2
      (bind _object (Utilities|AsyncLoadAsset DissolveNiagaraSystem)
        (:Completed
          (bind _asniagara_system (Utilities|Casting|CastToNiagaraSystem _object))
          (bind _returnvalue_3 (Niagara|SpawnSystemAttached _asniagara_system (Variables|Character|GetMesh) "None" "0, 0, 0" "0, 0, 0" "KeepRelativeOffset" true))
          (bind _returnvalue_4 (Rendering|Material|CreateDynamicMaterialInstance _mesh 0 (Rendering|Material|GetMaterial _mesh 0) "None" :!class /Script/Engine.PrimitiveComponent))
          (bind _returnvalue_5 (Rendering|Material|GetVectorParameterValue _returnvalue_4 "DissolveEdgeColor" :!class /Script/Engine.MaterialInstanceDynamic))
          (Niagara|SetNiagaraVariable(LinearColor) _returnvalue_3 "DissolveParticleColor" _returnvalue_5)
          (Components|Timeline|SetPlayRate (Variables|Default|GetDissolveTimeline) (/ 1.0 (Variables|Default|GetTotalDissolveTime)))
          (bind _normalizedfloattrack (Timeline|DissolveTimeline Play)
            (:Update
              (Rendering|Material|SetScalarParameterValueonMaterials (Variables|Character|GetMesh) "DissolveAmount" _normalizedfloattrack)
              (Utilities|IsValid _returnvalue_2
                (:Is%20Valid
                  (Rendering|Material|SetScalarParameterValueonMaterials (Variables|/Script/Warrior.WarriorWeaponBase|GetWeaponMeshPtr _returnvalue_2) "DissolveAmount" _normalizedfloattrack))))
            (:Finished
              (Utilities|IsValid _returnvalue
                (:Is%20Valid
                  (Actor|DestroyActor _returnvalue))
                (:Is%20Not%20Valid
                  _))
              (Class|WarriorAbilitySystemComponent|TryActivateAbilitybyTag (Variables|Default|GetWarriorAbilitySystemComponentPtr) "(TagName=\"Enemy.Ability.SpawnStone\")" true)
              (Utilities|FlowControl|Delay 1e+01)
              (Actor|DestroyActor))))))))

(fn ConstructionScript)